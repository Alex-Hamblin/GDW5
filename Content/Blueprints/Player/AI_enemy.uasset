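; AI enemy pawn that moves toward the level's objective and can step through an array of waypoints.
; On BeginPlay it caches the first BP_Objective found and issues AIMoveTo toward it.
; Tick checks distance to the stored destination; when close, it increments the waypoint index and moves to that waypoint.
; The destination is only set by waypoint moves, and the index has no bounds check.
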(event Custom|MoveToNextWaypoint
  (bind _output (CallFunction|GetNextWaypoint))
  (bind _output_get (Variables|Default|SetDestiation (Transformation|GetActorLocation _output)))
  (AI|AIMoveTo self _output_get 0 5.0 false))

(event EventBeginPlay
  (CallFunction|LocateObjective)
  (AI|AIMoveTo self "0, 0, 0" (Variables|Default|Getobjective) 5.0 false))

(event Collision|EventActorBeginOverlap
  (params (OtherActor :type Actor%20Object%20Reference)))

(event EventTick
  (params (DeltaSeconds :type Float%20%28single-precision%29))
  (if (<= (Math|Vector|Distance(Vector) (Variables|Default|GetDestiation) (Transformation|GetActorLocation)) 1e+02)
    (CallFunction|MovetoNextWaypoint)))

(fn ConstructionScript)

(fn LocateObjective
  (bind _outactors (Actor|GetAllActorsOfClass "/Game/Blueprints/Player/BP_Objective.BP_Objective_C"))
  (Variables|Default|Setobjective (Utilities|Array|Get(acopy) _outactors)))

(fn GetNextWaypoint
  (bind _output_get (Variables|Default|Setwaypoint%20index (+ (Variables|Default|Getwaypoint%20index) 1)))
  (return (Utilities|Array|Get(acopy) (Variables|Default|Getwaypoints) _output_get)))