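; BP_Turret is a turret that continuously tracks player 0's pawn and fires BP_bullet actors at it.
; Every Tick it turns the actor toward the player and sets the Arrow component to a random direction within a Cone half-angle around that aim, adding spread.
; A Delay on Tick throttles firing to a FireRate interval, reset on each Tick, and bullets spawn at the Arrow's world transform.
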(event EventBeginPlay)

(event Collision|EventActorBeginOverlap
  (params (OtherActor :type Actor%20Object%20Reference)))

(event EventTick
  (params (DeltaSeconds :type Float%20%28single-precision%29))
  (bind _returnvalue (Transformation|GetActorLocation))
  (bind _returnvalue_2 (Game|Player|GetPlayerPawn 0))
  (bind _returnvalue_3 (Transformation|GetActorLocation _returnvalue_2))
  (bind _returnvalue_4 (Math|Rotator|FindLookatRotation _returnvalue _returnvalue_3))
  (Transformation|SetWorldRotation (Variables|Default|GetArrow) (Math|Conversions|RotationFromXVector (Class|KismetMathLibrary|RandomUnitVectorinConeinRadians (Math|Rotator|GetRotationXVector _returnvalue_4) (Variables|Default|Getcone))) false false)
  (Transformation|SetActorRotation _returnvalue_4)
  (bind _output_get (Variables|Default|SetFireRate 0.2))
  (Utilities|FlowControl|Delay _output_get)
  (Game|SpawnActorfromClass "/Game/Blueprints/Player/BP_bullet.BP_bullet_C" (Transformation|GetWorldTransform (Variables|Default|GetArrow)) "Undefined" "MultiplyWithRoot" 0 0))

(fn ConstructionScript)